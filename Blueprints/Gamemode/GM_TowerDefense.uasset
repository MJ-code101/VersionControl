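; Tower defense game mode that runs enemy waves and decides when the player wins.
; Each wave spawns twice its number in skeletons at random BP_spawnpoint actors, plus a mutant from wave three onward.
; SkeletonKilled counts down the skeletons, then either ends the game after the final wave or starts a timed buy break before the next.
; Counts, round messages and win/lose results are pushed to the player character's UI.
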(event `self.ReceiveBeginPlay`
  ; event play set refs
  (`|ExecutionSequence`
    (:`then_0`
      (bind _outactors (`GameplayStatics.GetAllActorsOfClass` "/Game/core/Blueprints/Skeleton/BP_spawnpoint.BP_spawnpoint_C"))
      (set `self.SpawnPoints` _outactors)
      (`self.SpawnSkeletons`))
    (:`then_1`
      (bind _outactors_2 (`GameplayStatics.GetAllActorsOfClass` "/Game/core/Blueprints/BP_ThirdPersonCharacter.BP_ThirdPersonCharacter_C"))
      (set `self.CharacterRef` (`|GetArrayItem` _outactors_2)))))

(event `SpawnSkeletons`
  (bind _characterref (`self.CharacterRef`))
  ; Spawn skeleton in game
  (bind _output_get (set `self.Skeletontotal` (* (`self.CurrentWave`) 2)))
  (set `self.SkeletonLeft` _output_get)
  (for _ (range 1 (+ (`self.Skeletontotal`) 1))
    (`|SpawnActorFromClass` "/Game/core/Blueprints/Skeleton/BP_skeleton.BP_skeleton_C" (`KismetMathLibrary.MakeTransform` (`self.K2_GetActorLocation` (`KismetArrayLibrary.Array_Random` (`self.SpawnPoints`)))) "Undefined" "MultiplyWithRoot" null null))
  (`|ExecutionSequence`
    (:`then_0`
      (`/Engine/EditorBlueprintResources/StandardMacros.IsValid` _characterref
        (:`Is Valid`
          (message `/Game/core/Blueprints/Interfaces/BPI_SoldierCharacter.UpdateSkeletonUI` _characterref (`self.SkeletonLeft`) (`self.Skeletontotal`)))))
    (:`then_1`
      (if (>= (`self.CurrentWave`) 3)
        (`|SpawnActorFromClass` "/Game/core/Blueprints/Skeleton/BP_Mutant.BP_Mutant_C" (`KismetMathLibrary.MakeTransform` (`self.K2_GetActorLocation` (`KismetArrayLibrary.Array_Random` (`self.SpawnPoints`)))) "Undefined" "MultiplyWithRoot" null null)
        (message `/Game/core/Blueprints/Interfaces/BPI_SoldierCharacter.UpdateSkeletonUI` (`self.CharacterRef`) (+ (`self.SkeletonLeft`) 1) (+ (`self.Skeletontotal`) 1))))))

(event `/Game/core/Blueprints/Interfaces/BPI_TowerDefenseGameMode.SkeletonKilled`
  (bind _characterref (`self.CharacterRef`))
  ; Count Skeleton Killed
  (bind _result (`/Engine/EditorBlueprintResources/StandardMacros.DecrementInt` (`self.SkeletonLeft`))
    (:`  `
      (if (== _result 0)
        (`KismetSystemLibrary.PrintString` "All Skeletons are Killed, Next Wave Starting.")
        (`self.WaveIncrement`))
      (`/Engine/EditorBlueprintResources/StandardMacros.IsValid` _characterref
        (:`Is Valid`
          (message `/Game/core/Blueprints/Interfaces/BPI_SoldierCharacter.UpdateSkeletonUI` _characterref (`self.SkeletonLeft`) (`self.Skeletontotal`)))))))

(event `WaveIncrement`
  (bind _characterref (`self.CharacterRef`))
  ; Check if player won and start teh next wave
  (if (== (`self.CurrentWave`) (`self.MaxWaves`))
    (`/Game/core/Blueprints/Interfaces/BPI_TowerDefenseGameMode.GameOver` false)
    (else
      (`/Engine/EditorBlueprintResources/StandardMacros.IncrementInt` (`self.CurrentWave`)
        (:`  `
          (`self.PreRounTimer`)))))
  (`/Engine/EditorBlueprintResources/StandardMacros.IsValid` _characterref
    (:`Is Valid`
      (message `/Game/core/Blueprints/Interfaces/BPI_SoldierCharacter.UpdateWavesUI` _characterref (`self.CurrentWave`) (`self.MaxWaves`)))))

(event `PreRounTimer`
  (bind _characterref (`self.CharacterRef`))
  ; Countdown
  (`/Engine/EditorBlueprintResources/StandardMacros.IsValid` _characterref
    (:`Is Valid`
      (message `/Game/core/Blueprints/Interfaces/BPI_SoldierCharacter.NextRoundStarting` _characterref))
    (:`Is Not Valid`
      _))
  (`KismetSystemLibrary.K2_SetTimerDelegate` (delegate `StartNextWave`) 15.0))

(event `StartNextWave`
  (bind _characterref (`self.CharacterRef`))
  ; Countdown
  (`self.SpawnSkeletons`)
  (`/Engine/EditorBlueprintResources/StandardMacros.IsValid` _characterref
    (:`Is Valid`
      (message `/Game/core/Blueprints/Interfaces/BPI_SoldierCharacter.StopBuyMode` _characterref))))

(event `/Game/core/Blueprints/Interfaces/BPI_TowerDefenseGameMode.GameOver`
  (params (`LostGame?` :type Boolean))
  (bind _characterref (`self.CharacterRef`))
  ; Show Win or Lose Screen on Player Widget
  (`/Engine/EditorBlueprintResources/StandardMacros.IsValid` _characterref
    (:`Is Valid`
      (message `/Game/core/Blueprints/Interfaces/BPI_SoldierCharacter.WinOrLoseGame` _characterref (not `LostGame?`)))))

(fn `UserConstructionScript`)