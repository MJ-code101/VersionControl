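; BP_Mutant is a melee enemy that chases the player from spawn and usually drops a coin when killed.
; AIMoveTo success triggers an attack montage whose notify applies damage through a sphere overlap, then the chase restarts.
; Damage from non-Skeleton-tagged sources updates a health bar widget.
; Death enables mesh physics, plays a dying montage, notifies the game mode and destroys the actor after a delay.
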(event `self.ReceiveBeginPlay`
  ; if see character,30% chance of skeleton chasing the player
  (set `self.PlayerRef` (`GameplayStatics.GetPlayerPawn` 0))
  (`self.ChasePlayer `))

(event `ChasePlayer`
  ; Chase Player Evemt
  (if (and (not (`self.IsDead`)) (not (`self.ChasingPlayer?`)) (not (`self.IsChasingKeep`)) (not (`self.IsAttacking`)))
    (set `self.ChasingPlayer?` true)
    (`|AIMoveTo` self (0.0 0.0 0.0) (`self.PlayerRef`)
      (:`OnSuccess`
        (`self.AttackPlayerEvent`)))))

(event `AttackPlayerEvent`
  ; Attack Player
  (if (and (not (`self.IsDead`)) (not (`self.IsAttacking`)))
    (set `self.IsAttacking` true)
    (`|PlayMontage` (`self.Mesh`) "/Game/core/Blueprints/Skeleton/Mutant/Mutant_Animation/Attack.Attack"
      (:`OnCompleted`
        (set `self.IsAttacking` false :!label _label)
        (set `self.ChasingPlayer?` false)
        (`self.ChasePlayer `))
      (:`OnInterrupted`
        (goto _label))
      (:`OnNotifyBegin`
        (bind (_outactors _returnvalue) (`KismetSystemLibrary.SphereOverlapActors` (`SceneComponent.K2_GetComponentLocation` (`self.Arrow1`)) 100.0 (`|MakeArray` "ObjectTypeQuery1" "ObjectTypeQuery2" "ObjectTypeQuery3" :!type "EObjectTypeQuery Enum") null (`|MakeArray` self :!type "Actor Object Reference")))
        (if _returnvalue
          (for _array_element _outactors
            (`GameplayStatics.ApplyDamage` _array_element 25.0 null self "/Script/Engine.DamageType")))))))

(event `self.ReceiveAnyDamage`
  (params (Damage :type "Float (single-precision)") (DamageType :type "DamageType Object Reference") (InstigatedBy :type "Controller Object Reference") (DamageCauser :type "Actor Object Reference"))
  ; Skeleton Receive Damage Event
  (if (not (`self.ActorHasTag` DamageCauser "Skeleton"))
    (if (`self.IsDead`)
      _
      (elif (<= (- (`self.Health`) Damage) 0.0)
        (set `self.Health` (- (`self.Health`) Damage))
        (message `/Game/core/Blueprints/Interfaces/BPI_HealthBarInterface.HideHealthBar` (`WidgetComponent.GetUserWidgetObject` (`self.Widget`)))
        (`self.Skeleton Death`)
        (else
          (bind _output_get (set `self.Health` (- (`self.Health`) Damage)))
          (message `/Game/core/Blueprints/Interfaces/BPI_HealthBarInterface.UpdateHealth` (`WidgetComponent.GetUserWidgetObject` (`self.Widget`)) _output_get))))))

(event `Skeleton Death`
  (bind _charactermovement (`self.CharacterMovement`))
  ; Skeleton Death Event
  (set `self.IsDead` true)
  (`PrimitiveComponent.SetSimulatePhysics` (`self.Mesh`) true)
  (`PrimitiveComponent.SetCollisionResponseToChannel` (`self.Mesh`) "ECC_Pawn" "ECR_Overlap")
  (`PrimitiveComponent.SetCollisionResponseToChannel` (`self.CapsuleComponent`) "ECC_Pawn" "ECR_Overlap")
  (`PrimitiveComponent.SetCollisionResponseToChannel` (`self.Mesh`) "ECC_Camera" "ECR_Overlap")
  (`PrimitiveComponent.SetCollisionResponseToChannel` (`self.CapsuleComponent`) "ECC_Camera" "ECR_Overlap")
  (`MovementComponent.StopMovementImmediately` _charactermovement)
  (`CharacterMovementComponent.DisableMovement` _charactermovement)
  (`|PlayMontage` (`self.Mesh`) "/Game/core/Blueprints/Skeleton/Mutant/Mutant_Animation/Mutant_Dying_MutantMesh_Anim_Montage.Mutant_Dying_MutantMesh_Anim_Montage"
    (:`then`
      (message `/Game/core/Blueprints/Interfaces/BPI_TowerDefenseGameMode.SkeletonKilled` (`GameplayStatics.GetGameMode`))
      (`self.SpawnCoin`)
      (`KismetSystemLibrary.Delay` 3.0)
      (`self.K2_DestroyActor`))))

(event `SpawnCoin`
  ; Spawn point pickup
  (if (`KismetMathLibrary.RandomBoolWithWeight` 0.9)
    (`|SpawnActorFromClass` "/Game/core/Blueprints/Pickups/Bp_Coinpickup.Bp_Coinpickup_C" (`KismetMathLibrary.MakeTransform` (+ (`SceneComponent.K2_GetComponentLocation` (`self.CapsuleComponent`)) (0.0 0.0 0.0))) "Undefined" "MultiplyWithRoot" null null)))

(fn `GetIsSkeletonDead?`
  (returns (`IsDead?` :type Boolean))
  (return (`self.IsDead`)))

(fn `UserConstructionScript`)