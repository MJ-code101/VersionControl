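; Turret cannon actor that automatically targets and shoots pawns tagged Skeleton.
; PawnSensing locks onto the first seen skeleton, starting looping tracking and firing timers.
; Tracking interpolates yaw toward the target and releases it only once the pawn is invalid.
; Firing periodically spawns BP_CannonBall at the Arrow's transform, stopping when the skeleton reports dead or the target is lost.
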(event `self.PawnSensing.OnSeePawn`
  (params (Pawn :type "Pawn Object Reference"))
  ; Event See Target
  (if (`self.ActorHasTag` Pawn "Skeleton")
    (`/Engine/EditorBlueprintResources/StandardMacros.IsValid` Pawn
      (:`Is Valid`
        (if (not (`self.HasTarget?`))
          (set `self.HasTarget?` true)
          (set `self.TargertPawn` Pawn)
          (`self.TrackTarget`)
          (`self.FireLoop`))))))

(event `TrackTarget`
  ; Rotate Cannon To Face Target
  (bind _returnvalue (`KismetSystemLibrary.K2_SetTimerDelegate` (delegate `MoveTurret`) 0.05 true true))
  (set `self.TimerRef` _returnvalue))

(event `MoveTurret`
  (bind _targertpawn (`self.TargertPawn`))
  (bind (_returnvalue_roll _returnvalue_pitch _returnvalue_yaw) (`KismetMathLibrary.BreakRotator` (`KismetMathLibrary.RInterpTo` (`self.K2_GetActorRotation`) (`KismetMathLibrary.FindLookAtRotation` (`self.K2_GetActorLocation`) (`self.K2_GetActorLocation` _targertpawn)) (`GameplayStatics.GetWorldDeltaSeconds`) 100.0)))
  ; Rotate Cannon To Face Target
  (`/Engine/EditorBlueprintResources/StandardMacros.IsValid` _targertpawn
    (:`Is Valid`
      (`self.K2_SetActorRotation` (`KismetMathLibrary.MakeRotator` 0.0 0.0 _returnvalue_yaw)))
    (:`Is Not Valid`
      (`KismetSystemLibrary.K2_ClearAndInvalidateTimerHandle` (`self.TimerRef`))
      (set `self.HasTarget?` false))))

(event `FireLoop`
  ; Fire Loop Logic
  (bind _returnvalue (`KismetSystemLibrary.K2_SetTimerDelegate` (delegate `FireCannon`) 4.0 true))
  (set `self.FireTimerRef` _returnvalue))

(event `FireCannon`
  ; Fire Loop Logic
  (if (`self.HasTarget?`)
    (bind _targertpawn (`self.TargertPawn`)
      (:`then`
        (bind _isdead_ (message `/Game/core/Blueprints/Interfaces/BPI_SkeletoCharactern.GetIsSkeletonDead?` _targertpawn))
        (if _isdead_
          (`KismetSystemLibrary.K2_ClearAndInvalidateTimerHandle` (`self.FireTimerRef`))
          (else
            (`|SpawnActorFromClass` "/Game/core/Blueprints/Items/BP_CannonBall.BP_CannonBall_C" (`SceneComponent.K2_GetComponentToWorld` (`self.Arrow`)) "Undefined" "MultiplyWithRoot" null null))))
      (:`else`
        (`KismetSystemLibrary.K2_ClearAndInvalidateTimerHandle` (`self.FireTimerRef`) :!label _label)))
    (else
      (goto _label))))

(fn `UserConstructionScript`)